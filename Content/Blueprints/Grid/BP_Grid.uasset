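; Tile grid for click-to-hop character movement, built in the Construction Script as spaced static mesh components.
; Tiles near the selected character are highlighted as available by a distance check.
; A click stores the hop location, then either warns on the HUD if a character overlaps the tile or highlights it, shows confirmation UI and notifies controller and character.
; Available tiles temporarily leave GridTiles to keep their highlight until reset.
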(event Custom|Clear%20SelectedTileMaterial
  (Rendering|Material|SetMaterial (Variables|Default|GetHitTile) 0 (Variables|Default|GetDefaultTileMaterial)))

(event Custom|SetAvailableTileMaterials
  ;[1 1 1] Set available tiles materials
  (Utilities|Array|Clear (Variables|Default|GetAvailableTiles))
  (bind _astop_down_controller (Utilities|Casting|CastToTopDownController (Game|GetPlayerController 0)))
  (for _array_element (Variables|Default|GetGridTiles)
    (if (< (Math|Vector|Distance(Vector) (Transformation|GetWorldLocation _array_element) (Transformation|GetActorLocation (Variables|/Game/Blueprints/TopDownController.TopDownController_C|GetSelectedCharacter _astop_down_controller))) 3e+02)
      (Rendering|Material|SetMaterial _array_element 0 (Variables|Default|GetAvailableTileMaterial))
      (Utilities|Array|Add (Variables|Default|GetAvailableTiles) _array_element))))

(event Custom|ResetTileMaterialsDefault
  ;[1 1 1] Reset tile materials
  (for _array_element (Variables|Default|GetAvailableTiles)
    (Utilities|Array|Add (Variables|Default|GetGridTiles) _array_element))
  (for _array_element_2 (Variables|Default|GetGridTiles)
    (Rendering|Material|SetMaterial _array_element_2 0 (Variables|Default|GetDefaultTileMaterial))))

(event EventClicked
  (params (HitLocation :type Vector :default "0, 0, 0") (SelectedCharacter :type Actor%20Object%20Reference) (HitComponent :type Primitive%20Component%20Object%20Reference))
  (Variables|Default|SetHitLocation HitLocation)
  (Variables|Default|SetHitTile HitComponent)
  ;[1 1 1] Send Hop location to selected character
  (Utilities|IsValid SelectedCharacter ; Ignore Click if no selected character
    (:Is%20Valid
      (CallFunction|SetHopLocation SelectedCharacter (Variables|Default|GetHitLocation))
      ;[1 1 1] Check if spot is occupied
      (bind _hittileoverlapscharacter (CallFunction|CheckifHitTileOverlapsAnyCharacter))
      (if _hittileoverlapscharacter
        (Default|SpotOccupied (CallFunction|GetHUD))
        (else
          (Utilities|FlowControl|Sequence
            (:then_0
              ;[1 1 1] Show movement confirmation UI
              (CallFunction|SetConfirmationMovementUIVisibility "Visible"))
            (:then_1
              ;[1 1 1] Set Selected tile material
              (for _array_element (Variables|Default|GetAvailableTiles)
                (Utilities|Array|RemoveItem (Variables|Default|GetGridTiles) _array_element))
              (for _array_element_2 (Variables|Default|GetGridTiles)
                (Rendering|Material|SetMaterial _array_element_2 0 (Variables|Default|GetDefaultTileMaterial)))
              (Rendering|Material|SetMaterial (Variables|Default|GetHitTile) 0 (Variables|Default|GetSelectedTileMaterial)))
            (:then_2
              ;[1 1 1] Set Character is confirming movement
              (bind _astop_down_controller (Utilities|Casting|CastToTopDownController (Game|GetPlayerController 0)))
              (Variables|/Game/Blueprints/TopDownController.TopDownController_C|SetIsCharacterConfirmingMovement _astop_down_controller true))
            (:then_3
              ;[1 1 1] Make selected character look at
              (Default|HopLocationSelected (Variables|Default|GetSelectedCharacter)))))))))

(fn ConstructionScript
  (bind _spacing (Variables|Default|GetSpacing))
  ;[1 1 1] Create grid
  (for _index (range 0 (Variables|Default|GetGrid_X_AmountOfTiles))
    (for _index_2 (range 0 (Variables|Default|GetGrid_Y_AmountOfTiles))
      (bind _returnvalue (AddComponent|AddStaticMeshComponent false (Math|Transform|MakeTransform (Math|Vector|MakeVector (* _index _spacing) (* _index_2 _spacing) (Variables|Default|GetHeightFromRoot)) "0, 0, 0" "1,1,1")))
      (Utilities|Array|Add (Variables|Default|GetGridTiles) _returnvalue)
      ;[1 1 1] Create dynamic tile material
      (bind _returnvalue_2 (Rendering|Material|CreateDynamicMaterialInstance "/Game/Geometry/Meshes/CubeMaterial_Yellow.CubeMaterial_Yellow" "Color" "None" :!class /Script/Engine.KismetMaterialLibrary))
      (Variables|Default|SetDefaultTileMaterial _returnvalue_2)
      (for _array_element (Variables|Default|GetGridTiles)
        (Rendering|Material|SetMaterial _array_element 0 (Variables|Default|GetDefaultTileMaterial))))))

(fn CheckifHitTileOverlapsAnyCharacter
  (bind _outactors (Actor|GetAllActorsOfClass "/Game/Blueprints/Pawn/Character_BASE.Character_BASE_C"))
  (bind _array_element (Utilities|Array|ForEachLoopwithBreak _outactors :!label _label)
    (:LoopBody
      (if (Collision|IsOverlappingActor (Variables|Default|GetHitTile) _array_element :!class /Script/Engine.PrimitiveComponent)
        (Variables|Default|SetIsHitTileOverlapAnyCharacter true)
        (goto _label Break)
        (else
          (Variables|Default|SetIsHitTileOverlapAnyCharacter false))))
    (:Completed
      (return (Variables|Default|GetIsHitTileOverlapAnyCharacter)))))

(fn GetHUD
  (return (Variables|/Game/Blueprints/TopDownGameMode.TopDownGameMode_C|GetHUD (.AsTop%20Down%20Game%20Mode (Utilities|Casting|CastToTopDownGameMode (Game|GetGameMode))))))

(fn SetHopLocation
  (params (SelectedCharacter :type Object%20Object%20Reference) (HopLocation :type Vector))
  (bind _ascharacter_base (Utilities|Casting|CastToCharacter_BASE SelectedCharacter))
  (bind _output_get (Variables|Default|SetSelectedCharacter _ascharacter_base))
  (Variables|/Game/Blueprints/Pawn/Character_BASE.Character_BASE_C|SetHopLocation _output_get HopLocation))

(fn SetConfirmationMovementUIVisibility
  (params (InVisibility :type ESlateVisibility%20Enum :default "Visible"))
  (Widget|SetVisibility (Variables|/Game/Blueprints/UI/HUD_BP.HUD_BP_C|GetMovementConfirmation_BP (CallFunction|GetHUD)) InVisibility))