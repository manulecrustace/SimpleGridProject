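; Base character for click-to-move on a tile grid, with selection and confirmed hop movement.
; Clicking resets every character's selection, highlights this one, focuses the camera and shows available tiles through BP_Grid, unless a move awaits confirmation.
; Choosing a destination turns the character via a timeline; confirming starts a timeline hop with separately lerped height.
; Confirming or clearing resets tiles and selection, clears the controller's confirming flag and hides the HUD confirmation widget.
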(event Custom|CharacterMovementConfirmed
  (Utilities|FlowControl|Sequence
    (:then_0
      (|HopToLocation)
      ;[1 1 1] Clear Tile Selection
      (Default|ClearSelectedTileMaterial (Variables|Default|GetGrid))
      ;[1 1 1] Update location
      (Variables|/Game/Blueprints/TopDownController.TopDownController_C|SetSelectedCharacterLocation (Variables|Default|GetPlayerController) (Transformation|GetActorLocation))
      (CallFunction|GetCameraFocusedonActor)
      ;[1 1 1] Clear available tiles
      (Default|ResetTileMaterialsDefault (Variables|Default|GetGrid))
      ;[1 1 1] Unselect Character
      (bind _output_get (Variables|Default|SetIsSelected false))
      (CallFunction|UpdateMaterialonSelectionState _output_get))
    (:then_1
      ;[1 1 1] Character no longer confirming movement
      (Variables|/Game/Blueprints/TopDownController.TopDownController_C|SetIsCharacterConfirmingMovement (Variables|Default|GetPlayerController) false)
      ;[1 1 1] Hide confirmation UI
      (CallFunction|ChangeMovementConfirmationUIVisibility "Hidden"))))

(event Custom|CharacterMovementCleared
  ;[1 1 1] Reset tile material
  (Default|ResetTileMaterialsDefault (Variables|Default|GetGrid))
  ;[1 1 1] Unselect character
  (bind _output_get (Variables|Default|SetIsSelected false))
  (CallFunction|UpdateMaterialonSelectionState _output_get)
  ;[1 1 1] Character no longer confirming movement
  (Variables|/Game/Blueprints/TopDownController.TopDownController_C|SetIsCharacterConfirmingMovement (Variables|Default|GetPlayerController) false)
  ;[1 1 1] Hide confirmation UI
  (CallFunction|ChangeMovementConfirmationUIVisibility "Hidden"))

(event Custom|HopLocationSelected
  (|LookAtHopLocation))

(event EventBeginPlay
  (bind _astop_down_game_mode (Utilities|Casting|CastToTopDownGameMode (Game|GetGameMode)))
  (Variables|Default|SetHUD (Variables|/Game/Blueprints/TopDownGameMode.TopDownGameMode_C|GetHUD _astop_down_game_mode))
  (bind _returnvalue (Actor|GetActorOfClass "/Game/Blueprints/Grid/BP_Grid.BP_Grid_C"))
  (Variables|Default|SetGrid _returnvalue)
  (bind _astop_down_controller (Utilities|Casting|CastToTopDownController (Game|GetPlayerController 0)))
  (Variables|Default|SetPlayerController _astop_down_controller))

(event EventClicked
  (params (HitLocation :type Vector :default "0, 0, 0") (SelectedCharacter :type Actor%20Object%20Reference) (HitComponent :type Primitive%20Component%20Object%20Reference))
  ;[1 1 1] Do Nothing if Character is confirming movement
  (bind _ischaracterconfirmingmovement (CallFunction|GetIsCharacterConfirmingMovement))
  (if (not _ischaracterconfirmingmovement)
    ;[1 1 1] Remove selected color for all characters
    (bind _outactors (Actor|GetAllActorsOfClass "Character_BASE_C"))
    (for _array_element _outactors
      (bind _output_get (Variables|Character_BASE_C|SetIsSelected _array_element false))
      (CallFunction|UpdateMaterialonSelectionState _array_element _output_get)
      ;[1 1 1] Select actor
      (bind _output_get_2 (Variables|Default|SetIsSelected true))
      (CallFunction|UpdateMaterialonSelectionState _output_get_2)
      (CallFunction|GetCameraFocusedonActor)
      ;[1 1 1] Show available spots
      (Default|SetAvailableTileMaterials (Variables|Default|GetGrid)))))

(fn ConstructionScript
  (Rendering|Material|SetMaterial (Variables|Default|GetCharacterMesh) 0 (Variables|Default|GetNormalMaterial)))

(fn GetCameraFocusedonActor
  (bind _returnvalue (Actor|GetActorOfClass "/Game/Blueprints/Camera_BP.Camera_BP_C"))
  (Default|FocusonActor _returnvalue))

(fn UpdateMaterialonSelectionState
  (params (IsSelected :type Boolean))
  (Rendering|Material|SetMaterial (Variables|Default|GetCharacterMesh) 0 (select IsSelected (Variables|Default|GetSelectedMaterial) (Variables|Default|GetNormalMaterial))))

(fn ChangeMovementConfirmationUIVisibility
  (params (Visibility :type ESlateVisibility%20Enum :default "Visible"))
  (Widget|SetVisibility (Variables|/Game/Blueprints/UI/HUD_BP.HUD_BP_C|GetMovementConfirmation_BP (Variables|Default|GetHUD)) Visibility))

(fn GetIsCharacterConfirmingMovement
  (bind _astop_down_controller (Utilities|Casting|CastToTopDownController (Game|GetPlayerController 0)))
  (return (Variables|/Game/Blueprints/TopDownController.TopDownController_C|GetIsCharacterConfirmingMovement _astop_down_controller)))